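; BP_Button is a floor button that the player character triggers to operate a linked gate.
; Capsule overlap plays a Do Once-guarded timeline that moves the cylinder mesh, then opens BPGateRef if still pressed.
; End overlap clears the pressed flag, snaps the cylinder to a fixed offset and rejoins the gate check.
; The delayed close call sits behind a repeated pressed check, so it is unreachable as wired.
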(event OnComponentBeginOverlap(Capsule_Collision)
  (params (OverlappedComponent :type Primitive%20Component%20Object%20Reference) (OtherActor :type Actor%20Object%20Reference) (OtherComp :type Primitive%20Component%20Object%20Reference) (OtherBodyIndex :type Integer) (bFromSweep :type Boolean) (SweepResult :type Hit%20Result%20Structure%20%28by%20ref%29))
  (bind _bp_gateref (Variables|Default|GetBP_GateRef))
  (bind _staticmesh_cylinder (Variables|Default|GetStaticMesh_Cylinder))
  (bind _relativelocation (Variables|/Script/Engine.SceneComponent|GetRelativeLocation _staticmesh_cylinder))
  ;[0.2336 0.5156 0.5053] Button Down/Up
  (if (== OtherActor (Variables|Default|GetPlayerRef))
    (Variables|Default|SetbButtonIsDown true)
    (if (Collision|IsOverlappingActor (Variables|Default|GetCapsule_Collision) (Variables|Default|GetPlayerRef) :!class /Script/Engine.PrimitiveComponent)
      (Utilities|FlowControl|DoOnce false :!label _label
        (:Completed
          (bind _z (Timeline|Button_Down Play)
            (:Update
              (Transformation|SetRelativeLocation _staticmesh_cylinder (Math|Vector|MakeVector (.x _relativelocation) (.y _relativelocation) _z) false false)
              (Utilities|FlowControl|Delay 0.2)
              (goto _label Reset))
            (:Finished
              (if (Variables|Default|GetbButtonIsDown)
                ;[0.2344 0.2072 0.1367] Open/Close gate
                (if (Variables|Default|GetbButtonIsDown)
                  (Utilities|IsValid _bp_gateref
                    (:Is%20Valid
                      (Default|OpenGateEvent _bp_gateref)))
                  (else
                    (Utilities|IsValid _bp_gateref
                      (:Is%20Valid
                        (Utilities|FlowControl|Delay (Variables|Default|GetDuration))
                        (Default|CloseGateEvent _bp_gateref)))))))))))))

(event OnComponentEndOverlap(Capsule_Collision)
  (params (OverlappedComponent :type Primitive%20Component%20Object%20Reference) (OtherActor :type Actor%20Object%20Reference) (OtherComp :type Primitive%20Component%20Object%20Reference) (OtherBodyIndex :type Integer))
  (bind _bp_gateref (Variables|Default|GetBP_GateRef))
  ;[0.2336 0.5156 0.5053] Button Down/Up
  (if (== OtherActor (Variables|Default|GetPlayerRef))
    (Variables|Default|SetbButtonIsDown false)
    (Transformation|SetRelativeLocation (Variables|Default|GetStaticMesh_Cylinder) "0.000000,0.000000,-8.500000" false false)
    (if (Variables|Default|GetbButtonIsDown)
      ;[0.2344 0.2072 0.1367] Open/Close gate
      (if (Variables|Default|GetbButtonIsDown)
        (Utilities|IsValid _bp_gateref
          (:Is%20Valid
            (Default|OpenGateEvent _bp_gateref)))
        (else
          (Utilities|IsValid _bp_gateref
            (:Is%20Valid
              (Utilities|FlowControl|Delay (Variables|Default|GetDuration))
              (Default|CloseGateEvent _bp_gateref))))))))

(event EventBeginPlay
  ;[0.06966 0.125 0.1175] Create Player Ref
  (bind _asbp_third_person_character (Utilities|Casting|CastToBP_ThirdPersonCharacter (Game|GetPlayerCharacter 0)))
  (Variables|Default|SetPlayerRef _asbp_third_person_character))

(fn ConstructionScript)