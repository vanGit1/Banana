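; BP_FallingBlock is a block that drops when the player character overlaps its trigger box, then rises again.
; A fall Timeline drives the static mesh's world Z from an absolute height curve, keeping X and Y unchanged.
; When it finishes, box collision is disabled and, after a short delay, a rise Timeline moves the mesh before collision is re-enabled.
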(event OnComponentBeginOverlap(Box_Collison)
  (params (OverlappedComponent :type Primitive%20Component%20Object%20Reference) (OtherActor :type Actor%20Object%20Reference) (OtherComp :type Primitive%20Component%20Object%20Reference) (OtherBodyIndex :type Integer) (bFromSweep :type Boolean) (SweepResult :type Hit%20Result%20Structure%20%28by%20ref%29))
  (bind _staticmesh (Variables|Default|GetStaticMesh))
  (bind _staticmesh_2 (Variables|Default|GetStaticMesh))
  (bind _returnvalue (Transformation|GetWorldLocation _staticmesh_2))
  (bind _returnvalue_2 (Transformation|GetWorldLocation _staticmesh))
  ;[0.02076 0.04001 0.04167] Block Fall
  (if (== OtherActor (Variables|Default|GetPlayerRef))
    (Utilities|FlowControl|Delay 0.0)
    (bind _zheight (Timeline|BlockFall PlayFromStart)
      (:Update
        (Transformation|SetWorldLocation _staticmesh (Math|Vector|MakeVector (.x _returnvalue_2) (.y _returnvalue_2) _zheight) false false))
      (:Finished
        (Collision|SetCollisionEnabled (Variables|Default|GetBox_Collison) "NoCollision")
        (Utilities|FlowControl|Delay 0.5)
        (bind _zheight_2 (Timeline|BlockRise PlayFromStart)
          (:Update
            (Transformation|SetWorldLocation _staticmesh_2 (Math|Vector|MakeVector (.x _returnvalue) (.y _returnvalue) _zheight_2) false false))
          (:Finished
            (Collision|SetCollisionEnabled (Variables|Default|GetBox_Collison) "QueryAndPhysics")))))))

(event EventBeginPlay
  ;[0.06771 0.06771 0.06771] Create Player Ref
  (bind _asbp_third_person_character (Utilities|Casting|CastToBP_ThirdPersonCharacter (Game|GetPlayerCharacter 0)))
  (Variables|Default|SetPlayerRef _asbp_third_person_character))

(fn ConstructionScript)