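; BP_FireSpurt is a fire trap that damages the player while its flames are visible and the player stands inside its box.
; Player overlap shows the particle system after a short delay, and leaving hides it after a longer one.
; Tick checks particle visibility and overlap with the cached third-person character, then applies damage through a DoOnce that resets after a delay, producing periodic hits.
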(event OnComponentBeginOverlap(BoxCollision)
  (params (OverlappedComponent :type Primitive%20Component%20Object%20Reference) (OtherActor :type Actor%20Object%20Reference) (OtherComp :type Primitive%20Component%20Object%20Reference) (OtherBodyIndex :type Integer) (bFromSweep :type Boolean) (SweepResult :type Hit%20Result%20Structure%20%28by%20ref%29))
  ;[0.25 0.01302 0.01302] Activate Fire
  (if (== OtherActor (Variables|Default|GetPlayerRef))
    (Utilities|FlowControl|Delay 0.21) ; Время перед активацией ловушки
    (Rendering|SetVisibility (Variables|Default|GetParticleSystem) true false)))

(event OnComponentEndOverlap(BoxCollision)
  (params (OverlappedComponent :type Primitive%20Component%20Object%20Reference) (OtherActor :type Actor%20Object%20Reference) (OtherComp :type Primitive%20Component%20Object%20Reference) (OtherBodyIndex :type Integer))
  ;[0.04688 0.00257 0.00257] Deactivate Fire
  (if (== OtherActor (Variables|Default|GetPlayerRef))
    (Utilities|FlowControl|Delay 2.0)
    (Rendering|SetVisibility (Variables|Default|GetParticleSystem) false false)))

(event EventBeginPlay
  ;[0.0402 0.05734 0.06771] Create Player reference
  (bind _asbp_third_person_character (Utilities|Casting|CastToBP_ThirdPersonCharacter (Game|GetPlayerCharacter 0)))
  (Variables|Default|SetPlayerRef _asbp_third_person_character))

(event EventTick
  (params (DeltaSeconds :type Float%20%28single-precision%29))
  (if (Rendering|IsVisible (Variables|Default|GetParticleSystem))
    (if (Collision|IsOverlappingActor (Variables|Default|GetBoxCollision) (Variables|Default|GetPlayerRef) :!class /Script/Engine.PrimitiveComponent)
      (Utilities|FlowControl|DoOnce false :!label _label
        (:Completed
          (Game|Damage|ApplyDamage (Variables|Default|GetPlayerRef) 1e+01 0 0)
          (Utilities|FlowControl|Delay 0.75)
          (goto _label Reset))))))

(fn ConstructionScript)