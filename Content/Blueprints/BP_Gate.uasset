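; BP_Gate is a gate actor that opens and closes by moving its mesh vertically.
; OpenGate_Event and CloseGate_Event use the IsOpen flag to ignore redundant requests, then play the OpenGate timeline from the start or reverse it from the end.
; The timeline's ZHeight track sets the mesh's absolute world Z on each update, preserving X and Y, so the track values are not relative to the gate's placement.
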(event Custom|CloseGate_Event
  (bind _staticmesh_gate (Variables|Default|GetStaticMesh_Gate))
  (bind _returnvalue (Transformation|GetWorldLocation _staticmesh_gate))
  (if (Variables|Default|GetIsOpen) ; Если ворота открыты,\n(IsOpen = true)\nто можно закрыть их
    (Variables|Default|SetIsOpen false)
    (bind _zheight (Timeline|OpenGate ReverseFromEnd)
      (:Update
        (Transformation|SetWorldLocation _staticmesh_gate (Math|Vector|MakeVector (.x _returnvalue) (.y _returnvalue) _zheight) false false)))))

(event Custom|OpenGate_Event
  (bind _staticmesh_gate (Variables|Default|GetStaticMesh_Gate))
  (bind _returnvalue (Transformation|GetWorldLocation _staticmesh_gate))
  (if (not (Variables|Default|GetIsOpen)) ; Проверяем открыты\nли ворота, если\nэто так,то ничего\n не делать.
    (Variables|Default|SetIsOpen true)
    (bind _zheight (Timeline|OpenGate PlayFromStart)
      (:Update
        (Transformation|SetWorldLocation _staticmesh_gate (Math|Vector|MakeVector (.x _returnvalue) (.y _returnvalue) _zheight) false false)))))

(fn ConstructionScript)