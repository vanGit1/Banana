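; BP_HealthPickUp is a pickup actor that restores health to the player character.
; It caches the player as a BP_ThirdPersonCharacter on BeginPlay.
; When that player overlaps its Sphere, it adds its health amount to CurrentHealth with a hard-coded clamp, prints the new value and destroys itself.
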(event OnComponentBeginOverlap(Sphere)
  (params (OverlappedComponent :type Primitive%20Component%20Object%20Reference) (OtherActor :type Actor%20Object%20Reference) (OtherComp :type Primitive%20Component%20Object%20Reference) (OtherBodyIndex :type Integer) (bFromSweep :type Boolean) (SweepResult :type Hit%20Result%20Structure%20%28by%20ref%29))
  (bind _playerref (Variables|Default|GetPlayerRef))
  ;[0.07102 0.1146 0.07355] Health PickUP
  (if (== OtherActor _playerref)
    (bind _output_get (Variables|/Game/Blueprints/BP_ThirdPersonCharacter.BP_ThirdPersonCharacter_C|SetCurrentHealth _playerref (Math|Float|Clamp(Float) (+ (Variables|/Game/Blueprints/BP_ThirdPersonCharacter.BP_ThirdPersonCharacter_C|GetCurrentHealth (Variables|Default|GetPlayerRef)) (Variables|Default|GetHealthAamount)) 0.0 1e+02)))
    (Development|PrintString (Utilities|String|ToString(Float) _output_get))
    (Actor|DestroyActor)))

(event EventBeginPlay
  ;[0.0625 0.0625 0.0625] Create Player Ref
  (bind _asbp_third_person_character (Utilities|Casting|CastToBP_ThirdPersonCharacter (Game|GetPlayerCharacter 0)))
  (Variables|Default|SetPlayerRef _asbp_third_person_character))

(fn ConstructionScript)